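; BP_Player is a player pawn Blueprint that provides basic look and movement functions.
; InputTurn and InputLookUp pass axis values to controller yaw and pitch.
; Move applies movement input along the forward or right vector of a yaw-only rotation, chosen by a boolean, so pitch does not affect direction.
; The event graph and construction script are empty, and no input bindings appear here.
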(fn `InputLookUp`
  (params (`Y Axis` :type "Float (double-precision)"))
  (`self.AddControllerPitchInput` `Y Axis`))

(fn `InputTurn`
  (params (`X Axis` :type "Float (double-precision)"))
  (`self.AddControllerYawInput` `X Axis`))

(fn `Move`
  (params (bIsForward :type Boolean) (AxisValue :type "Float (double-precision)"))
  (bind _yaw_only_rotation (`/Game/Blueprints/Util/MathUtils.GetYawOnlyRotation` self))
  (if bIsForward
    (`self.AddMovementInput` (`KismetMathLibrary.GetForwardVector` _yaw_only_rotation) (`local.AxisValue`))
    (else
      (`self.AddMovementInput` (`KismetMathLibrary.GetRightVector` _yaw_only_rotation) (`local.AxisValue`)))))

(fn `UserConstructionScript`)